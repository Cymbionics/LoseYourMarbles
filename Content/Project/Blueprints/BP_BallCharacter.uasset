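; Player ball character, driven by Enhanced Input and an MPU motion sensor read through BP_SerialPort.
; A timer polls the sensor, Data parses the readings, and Tick turns rotation into movement, jumping and ball spin; C recalibrates.
; It also manages HUD, level-end and win widgets, counts coins, and computes waypoint yaw toward the LevelChanger.
; Acceleration is parsed but never applied, and several older control snippets sit disconnected.
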(event `/Game/Project/Blueprints/BPI_Movement.LongitudinalMovement`
  (params (SerialPort :type "/Game/Student/BP_SerialPort Object Reference"))
  ;[1 0.8894 0 0.25] Movement
)

(event `EnhancedInput|/Game/Project/Controller/Inputs/IA_Look`
  (params (ActionValue :type "Vector2D Structure") (ElapsedSeconds :type "Float (double-precision)") (TriggeredSeconds :type "Float (double-precision)") (InputAction :type "InputAction Object Reference" :default "/Game/Project/Controller/Inputs/IA_Look.IA_Look"))
  ;[0 1 0.01606] Controls
)

(event `/Game/Project/Blueprints/BPI_Movement.LateralMovement`
  (params (SerialPort :type "/Game/Student/BP_SerialPort Object Reference"))
  ;[1 0.8894 0 0.25] Movement
)

(event `EnhancedInput|/Game/Project/Controller/Inputs/IA_MoveForward`
  (params (ActionValue :type "Float (double-precision)") (ElapsedSeconds :type "Float (double-precision)") (TriggeredSeconds :type "Float (double-precision)") (InputAction :type "InputAction Object Reference" :default "/Game/Project/Controller/Inputs/IA_MoveForward.IA_MoveForward"))
  (bind (_returnvalue_roll _returnvalue_pitch _returnvalue_yaw) (`KismetMathLibrary.BreakRotator` (`self.GetControlRotation`)))
  ;[0 1 0.01606] Controls
  (:`Triggered`
    (`self.AddMovementInput` (`KismetMathLibrary.GetForwardVector` (`KismetMathLibrary.MakeRotator` 0.0 0.0 _returnvalue_yaw)) ActionValue)
    (bind _output_get (set `self.CurrentSpeed` 200.0))
    (set `self.RotationSpeed` (* _output_get -0.02))
    (`SceneComponent.K2_AddLocalRotation` (`self.BallBody`) (`KismetMathLibrary.MakeRotator` 0.0 (`self.RotationSpeed`)) false false))
  (:`Completed`
    (set `self.CurrentSpeed` 0.0 :!label _label)))

(event `/Game/Project/Blueprints/BPI_Movement.VerticalMovement`
  (params (SerialPort :type "/Game/Student/BP_SerialPort Object Reference"))
  ;[1 0.8894 0 0.25] Movement
)

(event `EnhancedInput|/Game/Project/Controller/Inputs/IA_MoveSides`
  (params (ActionValue :type "Float (double-precision)") (ElapsedSeconds :type "Float (double-precision)") (TriggeredSeconds :type "Float (double-precision)") (InputAction :type "InputAction Object Reference" :default "/Game/Project/Controller/Inputs/IA_MoveSides.IA_MoveSides"))
  (bind (_returnvalue_roll _returnvalue_pitch _returnvalue_yaw) (`KismetMathLibrary.BreakRotator` (`self.GetControlRotation`)))
  ;[0 1 0.01606] Controls
  (:`Triggered`
    (`self.AddMovementInput` (`KismetMathLibrary.GetRightVector` (`KismetMathLibrary.MakeRotator` 0.0 0.0 _returnvalue_yaw)) ActionValue)
    (bind _output_get (set `self.CurrentSpeed` 200.0))
    (set `self.RotationSpeed` (* _output_get -0.02))
    (`SceneComponent.K2_AddLocalRotation` (`self.BallBody`) (`KismetMathLibrary.MakeRotator` (`self.RotationSpeed`)) false false))
  (:`Completed`
    (goto _label)))

(event `EnhancedInput|/Game/Project/Controller/Inputs/IA_Jump`
  (params (ActionValue :type Boolean) (ElapsedSeconds :type "Float (double-precision)") (TriggeredSeconds :type "Float (double-precision)") (InputAction :type "InputAction Object Reference" :default "/Game/Project/Controller/Inputs/IA_Jump.IA_Jump"))
  ;[0 1 0.01606] Controls
  (:`Triggered`
    (`self.Jump`))
  (:`Completed`
    (`self.StopJumping`)))

(event `Waypoint`
  (bind (_returnvalue_roll _returnvalue_pitch _returnvalue_yaw) (`KismetMathLibrary.BreakRotator` (`KismetMathLibrary.FindLookAtRotation` (`SceneComponent.GetSocketLocation` (`self.PlayerCamera`) "None") (`self.EndLevelLocation`))))
  (bind _returnvalue (`GameplayStatics.GetActorOfClass` "/Game/Project/Blueprints/LevelChanger.LevelChanger_C"))
  (set `self.EndLevelLocation` (`self.K2_GetActorLocation` _returnvalue))
  (set `self.WaypointLocation` _returnvalue_yaw))

(event `poll`
  (`/Game/Student/BP_SerialPort.SendData` (`self.SerialPort`) "GetMotionData=1"))

(event `self.ReceiveBeginPlay`
  ;[0 0.5549 1] UI
  (`self.ActivateUI`)
  (bind _returnvalue (`GameplayStatics.GetActorOfClass` "/Game/Student/BP_SerialPort.BP_SerialPort_C"))
  (bind _output_get (set `self.SerialPort` _returnvalue))
  (add `/Game/Student/BP_SerialPort.DataReceived` _output_get (`|CreateDelegate` :!event `Data`))
  (`/Game/Student/BP_SerialPort.SendData` _output_get "CalibrateMotionSensor=1")
  (`self.EnableInput` (`GameplayStatics.GetPlayerController` 0)) ; Allows for calibration key input
  (`KismetSystemLibrary.K2_SetTimerDelegate` (delegate `poll`) 0.1 true)
  (`KismetSystemLibrary.K2_SetTimerDelegate` (delegate `Waypoint`) 0.01 true))

(event `ActivateUI`
  ;[0 0.5549 1] UI
  (bind _returnvalue (`|CreateWidget` "/Game/Project/UI/WBP_PlayerHud.WBP_PlayerHud_C"))
  (bind _output_get (set `self.PlayerHud` _returnvalue))
  (`UserWidget.AddToViewport` _output_get 0)
  (`/Game/Project/UI/WBP_PlayerHud.ActivateHud` (`self.PlayerHud`) self))

(event `PlayerLose`
  ;[0 0.5549 1] UI
  (`Widget.RemoveFromParent` (`self.PlayerHud`) :!label _label_2))

(event `LevelChangerUI`
  ;[0 0.5549 1] UI
  (bind _returnvalue (`|CreateWidget` "/Game/Project/UI/WBP_EndLevel.WBP_EndLevel_C"))
  (bind _output_get (set `self.EndLevelUIRef` _returnvalue))
  (`UserWidget.AddToViewport` _output_get 0)
  (`/Game/Project/UI/WBP_EndLevel.EndLevelUI` (`self.EndLevelUIRef`))
  (goto _label_2))

(event `EndScreen`
  ;[0 0.5549 1] UI
  (bind _returnvalue (`|CreateWidget` "/Game/Project/UI/WBP_WinScreen.WBP_WinScreen_C"))
  (`UserWidget.AddToViewport` _returnvalue 0)
  (`GameplayStatics.SetGamePaused` true))

(event `self.ReceiveTick`
  (params (DeltaSeconds :type "Float (single-precision)"))
  (`self.ApplyRotationMovementInputs`)
  ;[1 1 1] Does not translate well to movement?
  (`self.ApplyRotation`))

(event `Key|C`
  (params (Key :type "Key Structure"))
  (:`Pressed`
    (`KismetSystemLibrary.PrintString` "Calibrate Motion Sensor" true true (struct :`G` 1.0 :`B` 0.08531 :`A` 1.0) 5.0)
    (`/Game/Student/BP_SerialPort.SendData` (`self.SerialPort`) "CalibrateMotionSensor=1")))

(event `Data`
  (params (StringData :type String) (StringDataArray :type "Map of String to String"))
  (bind (_value _returnvalue) (`BlueprintMapLibrary.Map_Find` StringDataArray "MPU"))
  (if (`KismetStringLibrary.EqualEqual_StrStr` _value "ok")
    (`self.AccelerationData` StringDataArray)
    (`self.RotationData` StringDataArray)
    ;[1 1 1] Why is this node repeated?
    (`self.AccelerationData` StringDataArray)
    (elif _returnvalue
      (`KismetSystemLibrary.PrintString` _value) ; An Error With the MPU
    )))

(event `AccelerationData`
  (params (TargetMap :type "Map of String to String"))
  (set `self.AccX` (`KismetStringLibrary.Conv_StringToDouble` (`BlueprintMapLibrary.Map_Find` TargetMap "AccX")))
  (set `self.AccY` (`KismetStringLibrary.Conv_StringToDouble` (`BlueprintMapLibrary.Map_Find` TargetMap "AccY")))
  (set `self.AccZ` (`KismetStringLibrary.Conv_StringToDouble` (`BlueprintMapLibrary.Map_Find` TargetMap "AccZ"))))

(event `RotationData`
  (params (InputPin :type "Map of String to String"))
  (set `self.RotX` (`KismetStringLibrary.Conv_StringToDouble` (`BlueprintMapLibrary.Map_Find` InputPin "RotX")))
  (set `self.RotY` (`KismetStringLibrary.Conv_StringToDouble` (`BlueprintMapLibrary.Map_Find` InputPin "RotY")))
  (set `self.RotZ` (`KismetStringLibrary.Conv_StringToDouble` (`BlueprintMapLibrary.Map_Find` InputPin "RotZ"))))

(event `ApplyAcceleration`
  (if (`self.UseAccelerationData`)
    (`self.K2_SetActorLocation` (+ (`self.K2_GetActorLocation`) (`KismetMathLibrary.GreaterGreater_VectorRotator` (* (`KismetMathLibrary.MakeVector` (`self.AccX`) (`self.AccY`) (`self.AccZ`)) 0.001) (`self.K2_GetActorRotation`))))
    (`KismetSystemLibrary.PrintString` (`KismetTextLibrary.Conv_TextToString` (`|FormatText` "MPU - Acceleration \nAccX= {AccX} \nAccY= {AccY} \nAccZ= {AccZ}" (`self.AccX`) (`self.AccY`) (`self.AccZ`))) true false (struct :`G` 0.66 :`B` 1.0 :`A` 1.0) 2.0 "MPUAcceleration")))

(event `ApplyRotation`
  (bind _sensitivity (`self.Sensitivity`))
  (if (`self.UseRotationData`)
    (`SceneComponent.K2_AddWorldRotation` (`self.BallBody`) (`KismetMathLibrary.RLerp` (`KismetMathLibrary.MakeRotator` (/ (`self.RotX`) _sensitivity) (/ (`self.RotY`) _sensitivity) (/ (`self.RotZ`) _sensitivity)) (`self.K2_GetActorRotation`) 0.001 true) false false)
    (`KismetSystemLibrary.PrintString` (`KismetTextLibrary.Conv_TextToString` (`|FormatText` "MPU - Rotation \nRotX= {RotX} \nRotY= {RotY} \nRotZ= {RotZ} \nPress 'c' to calibrate" (`self.RotX`) (`self.RotY`) (`self.RotZ`))) true false (struct :`G` 0.66 :`B` 1.0 :`A` 1.0) 2.0 "MPURotation")))

(event `ApplyRotationMovementInputs`
  (bind (_returnvalue_roll _returnvalue_pitch _returnvalue_yaw) (`KismetMathLibrary.BreakRotator` (`self.GetControlRotation`)))
  (bind (_returnvalue_roll_2 _returnvalue_pitch_2 _returnvalue_yaw_2) (`KismetMathLibrary.BreakRotator` (`self.GetControlRotation`)))
  (`self.AddMovementInput` (`KismetMathLibrary.GetForwardVector` (`KismetMathLibrary.MakeRotator` 0.0 0.0 _returnvalue_yaw)) (`self.RotX`))
  (`self.AddMovementInput` (`KismetMathLibrary.GetRightVector` (`KismetMathLibrary.MakeRotator` 0.0 0.0 _returnvalue_yaw_2)) (`self.RotY`))
  (`KismetSystemLibrary.PrintString` (`KismetTextLibrary.Conv_TextToString` (`|FormatText` "MPU - Rotation \nRotX= {RotX} \nRotY= {RotY} \nRotZ= {RotZ} \nPress 'c' to calibrate" (`self.RotX`) (`self.RotY`) (`self.RotZ`))) true false (struct :`G` 0.66 :`B` 1.0 :`A` 1.0) 2.0 "MPURotation")
  (if (>= (* (`self.RotZ`) -1.0) 1.5)
    (`self.Jump`)
    (else
      (`self.StopJumping`))))

(event `/Game/Project/Blueprints/BPI_Pickup.CoinInterface`
  (params (Amount :type Integer))
  (bind _output_get (set `self.CollectedCoins` (+ Amount (`self.CollectedCoins`))))
  (`self.E_CoinUpdate` _output_get))

(fn `UserConstructionScript`)