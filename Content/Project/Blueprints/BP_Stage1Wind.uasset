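; BP_Stage1Wind is a wind hazard that pushes the player's ball character in a random horizontal direction.
; SetDirection triggers the character's wind warning, picks one of four directions through a random MultiGate, and starts a looping timer.
; StartWind passes the direction to CallSetWind and repeatedly launches the player until a delay clears the timer.
; BeginPlay is empty and the self-repeating SetDirection timer is disconnected, so nothing here starts the wind.
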(event `self.ReceiveBeginPlay`)

(event `SetDirection`
  (bind _asbp_ball_character (cast `/Game/Project/Blueprints/BP_BallCharacter` (`GameplayStatics.GetPlayerCharacter` 0)))
  (`/Game/Project/Blueprints/BP_BallCharacter.WindWarning` _asbp_ball_character)
  (`|MultiGate` true true
    (:`Out 0`
      (set `self.WindDirection` (0.0 500.0 -1.0)))
    (:`Out 1`
      (set `self.WindDirection` (500.0 0.0 -1.0)))
    (:`Out 2`
      (set `self.WindDirection` (-500.0 0.0 -1.0)))
    (:`Out 3`
      (set `self.WindDirection` (0.0 -500.0 -1.0))))
  (bind _returnvalue (`KismetSystemLibrary.K2_SetTimerDelegate` (delegate `Start Wind`) 0.2 true))
  (set `self.TimerReset` _returnvalue))

(event `Start Wind`
  (bind _winddirection (`self.WindDirection`))
  (`self.SetWind` _winddirection)
  (`Character.LaunchCharacter` (`GameplayStatics.GetPlayerCharacter` 0) _winddirection true true)
  (`KismetSystemLibrary.Delay` 5.0)
  (`KismetSystemLibrary.K2_ClearAndInvalidateTimerHandle` (`self.TimerReset`)))

(fn `UserConstructionScript`)