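; LevelChanger is a trigger actor that ends the level when the ball character reaches it.
; When BP_BallCharacter overlaps its Box, it calls that character's LevelChangerUI and disables input on the player character.
; It then plays a victory sound and opens the level named by NextLevel after a short delay.
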(event `self.Box.OnComponentBeginOverlap`
  (params (OverlappedComponent :type "PrimitiveComponent Object Reference") (OtherActor :type "Actor Object Reference") (OtherComp :type "PrimitiveComponent Object Reference") (OtherBodyIndex :type Integer) (bFromSweep :type Boolean) (SweepResult :type "HitResult Structure (by ref)"))
  (bind _asbp_ball_character (cast `/Game/Project/Blueprints/BP_BallCharacter` OtherActor))
  (`/Game/Project/Blueprints/BP_BallCharacter.LevelChangerUI` _asbp_ball_character)
  (`self.Stop Player Input`)
  (`self.Open Next Level`))

(event `Open Next Level`
  (`GameplayStatics.PlaySound2D` "/Game/Project/Sounds/SoundCues/SC_Victory.SC_Victory" 1.0 1.0 0.0 null null)
  (`KismetSystemLibrary.Delay` 3.0)
  (`GameplayStatics.OpenLevel` (`self.NextLevel`)))

(event `Stop Player Input`
  (`self.DisableInput` (`GameplayStatics.GetPlayerCharacter` 0) (`GameplayStatics.GetPlayerController` 0)))

(fn `UserConstructionScript`)